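; Compass manager component for the QuestMap system that drives the HUD compass and its waypoint marker.
; Initialize uses interface messages on the controller to cache the world map manager and the compass's dynamic material.
; Each tick pans the material by normalized control yaw plus a direction offset.
; It also shows and positions the marker from the yaw difference to the world map's waypoint actor, hiding it when none exists.
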(event EventTick
  (params (DeltaSeconds :type Float%20%28single-precision%29))
  (if (Variables|OperatingValues|GetInitialized?) ; Has this component been initialized?
    (CallFunction|Update) ; Update the compass every frame.
  ))

(event EventInitialize
  (params (Controller :type Player%20Controller%20Object%20Reference))
  (CallFunction|InitializeReferences Controller))

(fn Update
  (Utilities|IsValid (Variables|References|GetCompassMaterial) ; Is the material valid?
    (:Is%20Valid
      (Rendering|Material|SetScalarParameterValue (Variables|References|GetCompassMaterial) "PlayerInput" (+ (/ (.Yaw (Math|Rotator|BreakRotator (Pawn|GetControlRotation (Game|GetPlayerController 0) :!class /Script/Engine.Controller))) 3.6e+02) (Variables|QuestMap-WorldMapSettings|GetDirectionOffset)) :!class /Script/Engine.MaterialInstanceDynamic) ; Set the material panning based on the player rotation.
      (CallFunction|GetWaypointMarker) ; Get the waypoint marker for the compass
      (return))
    (:Is%20Not%20Valid
      (return))))

(fn InitializeReferences
  (params (PlayerController :type Player%20Controller%20Object%20Reference))
  (bind _output_get (LocalVariables|SetController PlayerController)) ; Store input for use.
  (bind _worldmapmanager (Class|BPIntQuestMapController|GetComponents(Message) _output_get)) ; Retrieve QuestMap components from controller.
  (Utilities|IsValid _worldmapmanager ; Was a valid world map manager found?
    (:Is%20Valid
      (Variables|References|SetManager-WorldMap _worldmapmanager) ; Store reference to world map manager.
    )
    (:Is%20Not%20Valid
      _))
  (bind _questmapmanager (Class|BPIntQuestMapController|GetQMManager(Message) (LocalVariables|GetController))) ; Retrieve reference to the manager  from the controller.
  (Utilities|IsValid _questmapmanager ; Does the player have a valid HUD?
    (:Is%20Valid
      (bind _compass (Class|BPIntQuestMapHUD|GetCompass(Message) _questmapmanager)) ; Retrieve a reference to the compass on the HUD.
      (Utilities|IsValid _compass ; Was a valid compass found?
        (:Is%20Valid
          (bind _returnvalue (Appearance|GetDynamicMaterial _compass :!class /Script/UMG.Image)) ; Retrieve dynamic material version of\nHUD compass.
          (Variables|References|SetCompassMaterial _returnvalue) ; Store compass material for use.
        )
        (:Is%20Not%20Valid
          _)))
    (:Is%20Not%20Valid
      _))
  (Variables|OperatingValues|SetInitialized? true) ; Update initialized state bool.
  (return))

(fn GetWaypointMarker
  (bind _returnvalue (Game|Player|GetPlayerPawn 0))
  (bind _waypoint (Class|BPIntQuestMapGeneric|GetWaypointActor(Message) (Variables|References|GetManager-WorldMap))) ; Retrieve a reference to the waypoint actor defined in the\nworldmap manager.
  (Utilities|IsValid _waypoint ; Is there currently a valid waypoint?
    (:Is%20Valid
      (Rendering|Material|SetScalarParameterValue (Variables|References|GetCompassMaterial) "MarkerSwitch" 1.0 :!class /Script/Engine.MaterialInstanceDynamic) ; Set the marker to visible.
      (bind _waypoint_2 (Class|BPIntQuestMapGeneric|GetWaypointActor(Message) (Variables|References|GetManager-WorldMap))) ; Retrieve a reference to the waypoint actor defined in the\nworldmap manager.
      (Rendering|Material|SetScalarParameterValue (Variables|References|GetCompassMaterial) "LocationInput" (+ (/ (- (.Yaw (Math|Rotator|BreakRotator (Pawn|GetControlRotation _returnvalue :!class /Script/Engine.Pawn))) (.Yaw (Math|Rotator|BreakRotator (Math|Rotator|FindLookatRotation (Transformation|GetActorLocation _returnvalue) (Transformation|GetActorLocation _waypoint_2))))) 3.6e+02) (Variables|QuestMap-WorldMapSettings|GetDirectionOffset)) :!class /Script/Engine.MaterialInstanceDynamic) ; Set the marker offset on the material.
      (return))
    (:Is%20Not%20Valid
      (Rendering|Material|SetScalarParameterValue (Variables|References|GetCompassMaterial) "MarkerSwitch" 0.0 :!class /Script/Engine.MaterialInstanceDynamic) ; No valid waypoint, so hide the marker.
      (return))))