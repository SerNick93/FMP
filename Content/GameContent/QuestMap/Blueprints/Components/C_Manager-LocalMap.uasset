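; QuestMap manager component that runs the player's local map, showing the active WorldLocation's map image with a player marker.
; Initialize caches the HUD widgets and dynamic materials, then checks for overlapped locations; toggling the map swaps its visibility with the compass.
; While open with a valid location, Tick rotates the marker through a material parameter and positions it by scaling the player's offset to the location's box or sphere bounds.
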(event EventTick
  (params (DeltaSeconds :type Float%20%28single-precision%29))
  (if (Variables|Default|GetInitialized?) ; Has this component been initialized?
    (if (Variables|Default|GetIsOpen) ; Is the local map currently open?
      (Utilities|IsValid (Variables|References|GetActiveLocation) ; Is there a valid active location?
        (:Is%20Valid
          (Marker-Player|UpdatePlayerRotation) ; Update player rotation on local map.
          (Marker-Player|UpdatePlayerLocation) ; Update player location on local map.
        )))))

(event EventInitialize
  (params (Controller :type Player%20Controller%20Object%20Reference))
  (Utility|InitializeReferences Controller) ; Initialize local map system.
)

(fn LocationCheck
  (for _array_element (Collision|GetOverlappingActors (Game|Player|GetPlayerPawn 0) "/Game/GameContent/QuestMap/Blueprints/Actors/WorldLocation.WorldLocation_C" :!class /Script/Engine.Actor) ; For all WorldLocation actors currently overlapping the player...
    (Default|PlayerIsOverlapping (.AsWorld%20Location (Utilities|Casting|CastToWorldLocation _array_element))) ; Call PlayerIsOverlapping function.
  )
  (return))

(fn InitializeReferences
  (params (PlayerController :type Player%20Controller%20Object%20Reference))
  (bind _output_get (LocalVariables|SetController PlayerController)) ; Store input for cleaner use.
  (bind _questmapmanager (Class|BPIntQuestMapController|GetQMManager(Message) _output_get))
  (Utilities|IsValid _questmapmanager ; Does the player controller have a valid\nHUD attached to it?
    (:Is%20Valid
      (bind (_compass _localmap) (Class|BPIntQuestMapHUD|GetWidgets(Message) _questmapmanager)) ; Retrieve QuestMap widgets from HUD.
      (Utilities|IsValid _compass ; Is there a valid compass widget?
        (:Is%20Valid
          (Variables|References|SetCompassWidget _compass) ; Store reference to compass widget.
        )
        (:Is%20Not%20Valid
          _))
      (bind _output_get_2 (Variables|References|SetLocalMapWidget _localmap)) ; Store reference to local map widget.
      (bind _output_get_3 (Variables|References|SetPlayerMarker (Variables|/Game/GameContent/QuestMap/Blueprints/Widgets/LocalMap.LocalMap_C|GetPlayerMarker _output_get_2))) ; Store reference to player marker.
      (bind _returnvalue (Appearance|GetDynamicMaterial (Variables|/Game/GameContent/QuestMap/Blueprints/Widgets/PlayerMarker.PlayerMarker_C|GetMarker _output_get_3) :!class /Script/UMG.Image)) ; Retrieve dynamic material version of\nplayer marker.
      (Variables|References|SetPlayerMarkerMaterial _returnvalue) ; Store reference to dynamic material version of player marker.
      (bind _returnvalue_2 (Appearance|GetDynamicMaterial (Variables|/Game/GameContent/QuestMap/Blueprints/Widgets/LocalMap_Image.LocalMap_Image_C|GetMap (Variables|/Game/GameContent/QuestMap/Blueprints/Widgets/LocalMap.LocalMap_C|GetLocalMap_Image (Variables|References|GetLocalMapWidget))) :!class /Script/UMG.Image)) ; Retrieve dynamic material version of\nlocal map image.
      (Variables|References|SetLocalMap _returnvalue_2) ; Store reference to dynamic material\nversion of local map image.
      (Utility|UpdateLocation) ; Update player location.
      (Utility|LocationCheck) ; Check if the player is in a location.
      (Variables|Default|SetIsOpen false) ; Update IsOpen state.
      (Variables|Default|SetInitialized? true) ; Update Initialized? state bool.
      (return))
    (:Is%20Not%20Valid
      (Development|PrintString "C_Manager-LocalMap: No valid HUD attached to player.") ; Notify of no valid HUD attached.
      (return))))

(fn AddPlayerMarkerInfo
  (bind _returnvalue (UserInterface|CreateWidget "/Game/GameContent/QuestMap/Blueprints/Widgets/PlayerInfo.PlayerInfo_C")) ; Create the tooltip widget.
  (Class|Widget|SetToolTip (Variables|References|GetPlayerMarker) _returnvalue) ; Associate the tooltip with the player marker.
  (return))

(fn Toggleon
  (bind _compasswidget (Variables|References|GetCompassWidget))
  (Utilities|IsValid _compasswidget ; Is there a valid compass widget?
    (:Is%20Valid
      (Widget|SetVisibility _compasswidget "Hidden") ; Hide the compass.
    )
    (:Is%20Not%20Valid
      _))
  (Widget|SetVisibility (Variables|References|GetLocalMapWidget) "Visible") ; Show the local map.
  (Variables|Default|SetIsOpen true) ; Update IsOpen state.
  (return))

(fn ToggleOff
  (bind _compasswidget (Variables|References|GetCompassWidget))
  (Utilities|IsValid _compasswidget ; Is there a valid compass widget?
    (:Is%20Valid
      (Widget|SetVisibility _compasswidget "Visible") ; Show the compass.
    )
    (:Is%20Not%20Valid
      _))
  (Widget|SetVisibility (Variables|References|GetLocalMapWidget) "Hidden") ; Hide the local map.
  (Variables|Default|SetIsOpen false) ; Update IsOpen state.
  (return))

(fn UpdateLocation
  (Utilities|IsValid (Variables|References|GetActiveLocation) ; Is the current location valid?
    (:Is%20Valid
      (Rendering|Material|SetTextureParameterValue (Variables|References|GetLocalMap) "MapImage" (Variables|/Game/GameContent/QuestMap/Blueprints/Actors/WorldLocation.WorldLocation_C|GetLocalMap (Variables|References|GetActiveLocation))) ; Set the current local map to the one associated with the active location.
      (Widget|SetVisibility (Variables|References|GetPlayerMarker) "Visible") ; Set the player marker to visible.
      (return))
    (:Is%20Not%20Valid
      (Rendering|Material|SetTextureParameterValue (Variables|References|GetLocalMap) "MapImage" "/Game/GameContent/QuestMap/Textures/Map/T_Map_Default.T_Map_Default") ; Clear the local map image.
      (Widget|SetVisibility (Variables|References|GetPlayerMarker) "Hidden") ; Set the player marker to hidden.
      (return))))

(fn UpdatePlayerRotation
  (Utilities|IsValid (Variables|References|GetPlayerMarkerMaterial) ; Is there a valid player marker material?
    (:Is%20Valid
      (Rendering|Material|SetScalarParameterValue (Variables|References|GetPlayerMarkerMaterial) "PlayerRotation" (/ (- 1.0 (.Yaw (Math|Rotator|BreakRotator (Pawn|GetControlRotation (Game|GetPlayerController 0) :!class /Script/Engine.Controller)))) 3.6e+02) :!class /Script/Engine.MaterialInstanceDynamic) ; Set the player rotation value in the material based on the player's control rotation converted to degrees.
      (return))
    (:Is%20Not%20Valid
      (return))))

(fn UpdatePlayerLocation
  (bind _returnvalue (Game|Player|GetPlayerPawn 0))
  (bind _activelocation (Variables|References|GetActiveLocation))
  (bind _returnvalue_2 (Transformation|GetActorLocation _returnvalue))
  (bind _defaultsceneroot (Variables|/Game/GameContent/QuestMap/Blueprints/Actors/WorldLocation.WorldLocation_C|GetDefaultSceneRoot _activelocation))
  (bind _returnvalue_3 (Transformation|GetWorldLocation _defaultsceneroot))
  (bind _returnvalue_4 (- _returnvalue_2 _returnvalue_3))
  (bind (_x _y) (Math|Vector|BreakVector _returnvalue_4))
  (LocalVariables|SetMapScale (Utility|GetMapScale)) ; Store map scale for reference.
  (Class|Widget|SetRenderTranslation (Variables|References|GetPlayerMarker) (+ (Math|Vector2D|MakeVector2D (/ _x (LocalVariables|GetMapScale)) (/ _y (LocalVariables|GetMapScale))) (- (/ (.X (Math|Vector2D|BreakVector2D (Class|Widget|GetDesiredSize (Variables|/Game/GameContent/QuestMap/Blueprints/Widgets/LocalMap.LocalMap_C|GetLocalMap_Image (Variables|References|GetLocalMapWidget))))) 2.0) (/ (.X (Math|Vector2D|BreakVector2D (Class|Widget|GetDesiredSize (Variables|References|GetPlayerMarker)))) 2.0)))) ; Set the player marker translation appropriately.
  (return))

(fn GetMapScale
  (bind _activelocation (Variables|References|GetActiveLocation))
  (bind _activelocation_2 (Variables|References|GetActiveLocation))
  (bind _activelocation_3 (Variables|References|GetActiveLocation))
  (bind _returnvalue (Transformation|GetActorTransform _activelocation))
  (bind _areacube (Variables|/Game/GameContent/QuestMap/Blueprints/Actors/WorldLocation.WorldLocation_C|GetAreaCube _activelocation_2))
  (bind _areasphere (Variables|/Game/GameContent/QuestMap/Blueprints/Actors/WorldLocation.WorldLocation_C|GetAreaSphere _activelocation_3))
  (bind _scale (Math|Transform|BreakTransform _returnvalue))
  (bind _boxextent (Variables|/Script/Engine.BoxComponent|GetBoxExtent _areacube))
  (bind _sphereradius (Variables|/Script/Engine.SphereComponent|GetSphereRadius _areasphere))
  (bind (_x _y) (Math|Vector|BreakVector _scale))
  (bind (_x_2 _y_2) (Math|Vector|BreakVector _boxextent))
  (LocalVariables|SetLocalMapCenter (/ (.X (Math|Vector2D|BreakVector2D (Class|Widget|GetDesiredSize (Variables|/Game/GameContent/QuestMap/Blueprints/Widgets/LocalMap.LocalMap_C|GetLocalMap_Image (Variables|References|GetLocalMapWidget))))) 2.0)) ; Measure the size of the Local Map image,\nand divide by 2 to get the center offset.
  (LocalVariables|SetLocationXScale _x) ; Stlore location X scale for use.
  (LocalVariables|SetLocationYScale _y) ; Stlore location Y scale for use.
  (if (Variables|/Game/GameContent/QuestMap/Blueprints/Actors/WorldLocation.WorldLocation_C|GetUseCubeCollision (Variables|References|GetActiveLocation)) ; Using sphere or cube collision?
    ;[1 1 1] Is the X or Y scale bigger?
    (if (> (LocalVariables|GetLocationXScale) (LocalVariables|GetLocationYScale))
      ;[1 1 1] Multiply the larger scale value by the longest side of the trigger, or in the case of a sphere, the radius.
      (LocalVariables|SetOutputScale (* (LocalVariables|GetLocationXScale) _x_2))
      (else
        (LocalVariables|SetOutputScale (* _y_2 (LocalVariables|GetLocationYScale)))))
    (elif (> (LocalVariables|GetLocationXScale) (LocalVariables|GetLocationYScale))
      (LocalVariables|SetOutputScale (* (LocalVariables|GetLocationXScale) _sphereradius))
      (else
        (LocalVariables|SetOutputScale (* _sphereradius (LocalVariables|GetLocationYScale))))))
  (return (/ (LocalVariables|GetOutputScale) (LocalVariables|GetLocalMapCenter))))

(fn SetLocation
  (params (ActiveLocation :type World%20Location%20Object%20Reference))
  (Variables|References|SetActiveLocation ActiveLocation)
  (return))

(fn GetActiveLocation
  (return (Variables|References|GetActiveLocation)))

(fn GetWaypointActor
  (return 0))