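; BP_Arrow is an arrow projectile for the player's bow that tilts along its flight path and disappears on contact.
; Each tick, ArrowAngle sets the actor's pitch from its velocity direction while keeping the current roll and yaw.
; Any overlap on the Capsule prints the other actor's name and destroys the arrow, with no damage applied in this graph.
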(event OnComponentBeginOverlap(Capsule)
  (params (OverlappedComponent :type Primitive%20Component%20Object%20Reference) (OtherActor :type Actor%20Object%20Reference) (OtherComp :type Primitive%20Component%20Object%20Reference) (OtherBodyIndex :type Integer) (bFromSweep :type Boolean) (SweepResult :type Hit%20Result%20Structure%20%28by%20ref%29))
  (Development|PrintString (Utilities|GetDisplayName OtherActor))
  (Actor|DestroyActor))

(event Custom|ArrowAngle
  (bind _returnvalue (Transformation|GetActorRotation))
  (bind (_roll _pitch _yaw) (Math|Rotator|BreakRotator _returnvalue))
  (Transformation|SetActorRotation (Math|Rotator|MakeRotator _roll (.Pitch (Math|Rotator|BreakRotator (Math|Rotator|MakeRotfromX (Transformation|GetVelocity)))) _yaw)))

(event EventBeginPlay)

(event EventTick
  (params (DeltaSeconds :type Float%20%28single-precision%29))
  (CallFunction|ArrowAngle))

(fn ConstructionScript)