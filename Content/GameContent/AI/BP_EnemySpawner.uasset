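; Enemy spawner actor that populates its Bound volume with ActorToSpawn pawns and keeps their count topped up.
; BeginPlay spawns SpawnAmount pawns, then a looping timer adds one whenever ActivePawns falls below that amount.
; SpawnEnemy picks random points in the bounds, traces downward against WorldStatic and spawns above the hit location.
; Each pawn gets a default controller and a SpawnPoint back-reference; removal from ActivePawns happens outside this Blueprint.
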(event EventBeginPlay
  (for _index (range 1 (Variables|Default|GetSpawnAmount))
    (CallFunction|SpawnEnemy))
  (Utilities|Time|SetTimerbyFunctionName 0 "RespawnEnemy" (Variables|Default|GetTimeUntilRespawn) true))

(fn ConstructionScript)

(fn SpawnEnemy
  (bind _bound (Variables|Default|GetBound))
  (bind (_origin _boxextent) (Collision|GetComponentBounds _bound))
  (bind _returnvalue (Math|Random|RandomPointinBoundingBox _origin _boxextent))
  (bind (_x _y _z) (Math|Vector|BreakVector _returnvalue))
  (bind _returnvalue_2 (+ _z 1e+03))
  (bind _returnvalue_3 (Math|Vector|MakeVector _x _y _returnvalue_2))
  (bind _outhit (Collision|LineTraceForObjects _returnvalue_3 (+ _returnvalue_3 (* (* (Transformation|GetActorUpVector) -1.0) 1.5e+03)) (Utilities|Array|MakeArray "ObjectTypeQuery1") false 0 "ForDuration"))
  (bind _returnvalue_4 (Game|SpawnActorfromClass (Variables|Default|GetActorToSpawn) (Math|Transform|MakeTransform (Math|Vector|MakeVector (.X (Math|Vector|BreakVector (.Location (Collision|BreakHitResult _outhit)))) (.Y (Math|Vector|BreakVector (.Location (Collision|BreakHitResult _outhit)))) (+ (.Z (Math|Vector|BreakVector (.Location (Collision|BreakHitResult _outhit)))) 1e+02)) (Math|Rotator|MakeRotator 0.0 0.0 (Math|Float|Clamp(Float) (Math|Random|RandomFloat) 0.0 3.6e+02))) "AdjustIfPossibleButAlwaysSpawn" 0 0))
  (Pawn|SpawnDefaultController _returnvalue_4)
  (Variables|/Game/GameContent/AI/Enemies/EnemyBaseClass.EnemyBaseClass_C|SetSpawnPoint _returnvalue_4 self)
  (Utilities|Array|Add (Variables|Default|GetActivePawns) _returnvalue_4))

(fn RespawnEnemy
  (if (< (Utilities|Array|Length (Variables|Default|GetActivePawns)) (Variables|Default|GetSpawnAmount))
    (CallFunction|SpawnEnemy)))