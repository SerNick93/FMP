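; Crystal Elemental enemy that fires spell projectiles at the player and plays a montage on death.
; Attack opens a gated, delay-throttled firing loop that StopShooting closes; shots take pitch from a look-at to the player, yaw and roll from RaycastOut.
; On BeginPlay, if the LostSoul quest is incomplete, it points its ObjectiveChecker at that quest and the YoungShaman.
; Tick runs a forward line trace whose result is unused.
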(event Custom|Shoot%20at%20player
  (bind _raycast_out (Variables|Default|GetRaycast%20out))
  (bind _rotator (CallFunction|CalculatePlayerRotation _raycast_out))
  (Game|SpawnActorfromClass "/Game/GameContent/AI/Enemies/CrystalElemental/SpellProjectile.SpellProjectile_C" (Math|Transform|MakeTransform (Transformation|GetWorldLocation _raycast_out) _rotator "0.500000,0.500000,0.500000") "Undefined" 0 0)
  (Animation|PlayAnimMontage "/Game/GameContent/AI/Enemies/CrystalElemental/Animations/A_CrystalELemental_SpellReady_Montage.A_CrystalELemental_SpellReady_Montage" 1.0 "None"))

(event EventBeginPlay
  (bind _objectivechecker (Variables|Default|GetObjectiveChecker))
  (bind _raycast_out (Variables|Default|GetRaycast%20out))
  (bind _newobjective (Variables|/Game/GameContent/DIALOGUE/DialogueTrees/ObjectiveCheckComponent/ObjectiveChecker.ObjectiveChecker_C|GetNewObjective _objectivechecker))
  (bind _output (Utilities|Array|Get(acopy) _newobjective))
  (|CallParentFunction)
  (Variables|Default|SetMaxRange (+ (Transformation|GetWorldLocation _raycast_out) (* (Math|Vector|GetForwardVector _raycast_out) 1e+02)))
  (bind _returnvalue (Actor|GetActorOfClass "/Game/GameContent/Quest/ActualQuests/LostSoul/LostSoul_Quest.LostSoul_Quest_C"))
  (bind _aslost_soul_quest (Utilities|Casting|CastToLostSoul_Quest _returnvalue))
  (if (not (Variables|/Game/GameContent/Quest/Quests/QuestParent.QuestParent_C|GetIsCompleted _aslost_soul_quest))
    (Variables|/Game/GameContent/DIALOGUE/DialogueTrees/ObjectiveCheckComponent/ObjectiveChecker.ObjectiveChecker_C|SetQuestToCheck _objectivechecker _returnvalue)
    (bind _returnvalue_2 (Actor|GetActorOfClass "/Game/GameContent/Quest/ActualQuests/LostSoul/YoungShaman.YoungShaman_C"))
    (Utilities|Array|SetArrayElem _newobjective 0 (Utilities|Struct|MakeStruct_ObjectiveData (.objectivetext _output) (.objectivetype _output) (.iscomplete _output) _returnvalue_2 (.number _output) (.objectivecollected _output)))
    (Development|PrintString (Utilities|GetDisplayName (.target (Utilities|Array|Get(acopy) _newobjective))))))

(event Collision|EventActorBeginOverlap
  (params (OtherActor :type Actor%20Object%20Reference)))

(event EventTick
  (params (DeltaSeconds :type Float%20%28single-precision%29))
  (bind _raycast_out (Variables|Default|GetRaycast%20out))
  (bind _returnvalue (Transformation|GetWorldLocation _raycast_out))
  (Collision|LineTraceByChannel _returnvalue (+ _returnvalue (* (Math|Vector|GetForwardVector _raycast_out) 1e+02)) "TraceTypeQuery1" false 0 "None"))

(event EventAttack
  (Development|PrintString "attack player")
  (Utilities|FlowControl|Sequence
    (:then_0
      (goto _label Open))
    (:then_1
      (if (Variables|Default|GetCanShoot)
        (Utilities|FlowControl|Gate true :!label _label
          (:Exit
            (CallFunction|ShootatPlayer)
            (Variables|Default|SetCanShoot false)
            (Utilities|FlowControl|Delay 1.5)
            (Variables|Default|SetCanShoot true)
            (goto _label)))))))

(event EventPlayerDeath
  (|CallParentFunction)
  (CallFunction|Death (Variables|Default|GetDeathMontage)))

(event EventStopShooting
  (if (Variables|Default|GetCanShoot)
    (Animation|StopAnimMontage "/Game/GameContent/AI/Enemies/CrystalElemental/Animations/A_CrystalELemental_SpellReady_Montage.A_CrystalELemental_SpellReady_Montage")
    (Utilities|FlowControl|Gate true) ; enters at Close
  ))

(fn ConstructionScript)

(fn OnRepIsDead
  (if (Variables|Default|GetIsDead_0)
    (CallFunction|Death)))

(fn CalculatePlayerRotation
  (params (NewParam1 :type Static%20Mesh%20Component%20Object%20Reference))
  (bind _returnvalue (Math|Vector|GetForwardVector NewParam1))
  (bind _returnvalue_2 (Math|Rotator|MakeRotfromX _returnvalue))
  (return (Math|Rotator|MakeRotator (.roll _returnvalue_2) (.pitch (Math|Rotator|FindLookatRotation _returnvalue (Transformation|GetActorLocation (Game|GetPlayerCharacter 0)))) (.yaw _returnvalue_2))))