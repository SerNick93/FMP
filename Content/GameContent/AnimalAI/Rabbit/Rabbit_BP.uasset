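; Rabbit AI actor that wanders the world or flees, driven by a self-repeating decision event started on BeginPlay.
; DecideNextAction picks a fast, long-range run if ShouldRun, otherwise a slow roam when neither hungry nor tired.
; Each AIMoveTo targets a random reachable point and re-enters the decision only on success.
; The random delay's branch is hard-wired to skip, ignoring SkipDelay, and hungry or tired states have no action.
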(event Custom|Decide%20Next%20Action
  (params (Skip%20Delay? :type Boolean))
  (if true
    _
    (else
      (Utilities|FlowControl|Delay (Math|Conversions|ToFloat(Integer) (Math|Random|RandomIntegerinRange 1 5)))))
  (if (Variables|Default|GetShould%20Run?)
    (CallFunction|RunAway)
    (elif (not (Variables|Default|GetIs%20Hungry?))
      (if (not (Variables|Default|GetIs%20Tired?))
        (CallFunction|RandomRoam)))))

(event Custom|Random%20Roam
  (Variables|/Script/Engine.CharacterMovementComponent|SetMaxWalkSpeed (Variables|Character|GetCharacterMovement) 1.5e+02)
  (AI|AIMoveTo self (.RandomLocation (AI|Navigation|GetRandomReachablePointinRadius (Transformation|GetActorLocation) 1e+04 0 0)) 0 5.0 false
    (:OnSuccess
      (CallFunction|DecideNextAction false))))

(event Custom|Run%20Away
  (Variables|/Script/Engine.CharacterMovementComponent|SetMaxWalkSpeed (Variables|Character|GetCharacterMovement) 6e+02)
  (AI|AIMoveTo self (.RandomLocation (AI|Navigation|GetRandomReachablePointinRadius (Transformation|GetActorLocation) (Math|Random|RandomFloatinRange 2e+04 3e+04) 0 0)) 0 5.0 false
    (:OnSuccess
      (CallFunction|DecideNextAction true))))

(event EventBeginPlay
  (CallFunction|DecideNextAction false))

(fn ConstructionScript)