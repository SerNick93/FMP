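; QuestMapManager is a PlayerController component that bootstraps the quest map and navigation UI for the local player.
; On BeginPlay it creates compass, local map and world map widgets according to which manager components are attached, hiding both maps by default.
; After a one-second delay it initializes every attached QuestMapComponent.
; It also exposes widget getters and toggles look/move input, plus cursor and mouse events for non-gamepad input.
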(event Custom|SetMovementState
  (params (Controller :type Player%20Controller%20Object%20Reference) (Disable? :type Boolean) (GamepadEvent :type Boolean))
  ;[1 1 1] Toggle player movement on/off.
  (Input|SetIgnoreLookInput Controller Disable?) ; Enable/disable look input.
  (Input|SetIgnoreMoveInput Controller Disable?) ; Enable/disable move input.
  (if (not GamepadEvent) ; Is this a gamepad event?
    (Variables|/Script/Engine.PlayerController|SetbEnableMouseOverEvents Controller Disable?) ; Enable/disable mouse over events.
    (Variables|/Script/Engine.PlayerController|SetbEnableClickEvents Controller Disable?) ; Enable/disable click events.
    (Variables|/Script/Engine.PlayerController|SetbShowMouseCursor Controller Disable?) ; Enable/disable mouse cursor.
  ))

(event EventBeginPlay
  ;[1 1 1] Initialize Quest Map and Navigation System.
  (bind _asplayer_controller (Utilities|Casting|CastToPlayerController (Components|GetOwner self)) ; Ensure owner is a player controller.
    (:then
      (if (Pawn|IsLocalController _asplayer_controller) ; Ensure initialization is client based only.
        (Variables|Default|SetPlayerController _asplayer_controller) ; Store controller reference for use.
        (CallFunction|CreateUI) ; Create the QuestMap UI.
        (Utilities|FlowControl|Delay 1.0) ; Delay to allow controller/character to intialize.
        (for _array_element (Actor|GetComponentsByClass (Variables|Default|GetPlayerController) "/Game/QuestMap/Blueprints/Components/QuestMapComponent.QuestMapComponent_C") ; For each component attached to the\ncontroller of the QuestMapComponent\nclass...
          (Default|Initialize _array_element (Variables|Default|GetPlayerController)) ; Execute initialize function, parsing a\nreference to the controller and this\nmanager component.
        )))
    (:CastFailed
      (Development|PrintString "QuestMapManager attached to actor not of PlayerController class.") ; Notify of casting error.
    )))

(fn CreateUI
  ;[1 1 1] Ensure prequisites are cleared on first run.
  (LocalVariables|SetHasCompass false) ; Clear HasCompass localstate.
  (LocalVariables|SetHasLocalMap false) ; Update HasLocalMap localstate.
  (LocalVariables|SetHasWorldMap false) ; Update HasWorlMap localstate.
  ;[1 1 1] Determine UI requirements.
  (for _array_element (Actor|GetComponentsByClass (Variables|Default|GetPlayerController) "/Game/QuestMap/Blueprints/Components/QuestMapComponent.QuestMapComponent_C") ; Retrieve a list of all quest map components attached to the player controller.
    (if (== (Utilities|GetClass _array_element) "/Game/QuestMap/Blueprints/Components/C_Manager-Compass.C_Manager-Compass_C") ; Is this current component a compass\nmanager?
      (LocalVariables|SetHasCompass true) ; Update HasCompass localstate.
      (elif (== (Utilities|GetClass _array_element) "/Game/QuestMap/Blueprints/Components/C_Manager-LocalMap.C_Manager-LocalMap_C") ; Is this current component a localmap\nmanager?
        (LocalVariables|SetHasLocalMap true) ; Update HasLocalMap localstate.
        (elif (== (Utilities|GetClass _array_element) "/Game/QuestMap/Blueprints/Components/C_Manager-LargeMap.C_Manager-LargeMap_C") ; Is this current component a worldmap\nmanager?
          (LocalVariables|SetHasWorldMap true) ; Update HasWorlMap localstate.
        ))))
  (if (LocalVariables|GetHasCompass) ; Do we need the compass UI?
    ;[1 1 1] Add the compass widget to viewport and save a reference for future use.
    (bind _returnvalue (UserInterface|CreateWidget "/Game/QuestMap/Blueprints/Widgets/Compass.Compass_C"))
    (UserInterface|Viewport|AddtoViewport _returnvalue 0)
    (Variables|Default|SetCompass _returnvalue))
  (if (LocalVariables|GetHasLocalMap) ; Do we need the LocalMap UI?
    ;[1 1 1] Add the local map widget to viewport and save a reference for future use. Set to hidden by default.
    (bind _returnvalue_2 (UserInterface|CreateWidget "/Game/QuestMap/Blueprints/Widgets/LocalMap.LocalMap_C"))
    (UserInterface|Viewport|AddtoViewport _returnvalue_2 0)
    (bind _output_get (Variables|Default|SetLocalMap _returnvalue_2))
    (Widget|SetVisibility _output_get "Hidden"))
  (if (LocalVariables|GetHasWorldMap) ; Do we need the WorldMap UI?
    ;[1 1 1] Add the world map widget to viewport and save a reference for future use. Set to hidden by default.
    (bind _returnvalue_3 (UserInterface|CreateWidget "/Game/QuestMap/Blueprints/Widgets/WorldMap.WorldMap_C"))
    (UserInterface|Viewport|AddtoViewport _returnvalue_3 0)
    (bind _output_get_2 (Variables|Default|SetWorldMap _returnvalue_3))
    (Widget|SetVisibility _output_get_2 "Hidden")
    (return)
    (else
      (return))))

(fn GetCompass
  (return (Variables|/Game/QuestMap/Blueprints/Widgets/Compass.Compass_C|GetCompass (Variables|Default|GetCompass))))

(fn GetWidgets
  (return (Variables|Default|GetCompass) (Variables|Default|GetLocalMap) (Variables|Default|GetWorldMap)))