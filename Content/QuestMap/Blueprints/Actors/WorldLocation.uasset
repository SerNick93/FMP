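; WorldLocation is a placeable quest map area that becomes discovered, displayed and announced for fast travel when the player first enters it.
; The construction script uses CollisionSwitch to enable either a box or sphere trigger, though its UseSphere flag actually selects the box.
; Overlap sets this location active on the local map manager and refreshes world map markers.
; Leaving clears it if still active.
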(event OnComponentBeginOverlap(AreaCube)
  (params (OverlappedComponent :type Primitive%20Component%20Object%20Reference) (OtherActor :type Actor%20Object%20Reference) (OtherComp :type Primitive%20Component%20Object%20Reference) (OtherBodyIndex :type Integer) (bFromSweep :type Boolean) (SweepResult :type Hit%20Result%20Structure%20%28by%20ref%29))
  ;[1 1 1] If overlapping actor is player, execute the overlap event.
  (if (== OtherActor (Variables|Components|GetPawn))
    (CallFunction|OverlapEvent)))

(event OnComponentBeginOverlap(AreaSphere)
  (params (OverlappedComponent :type Primitive%20Component%20Object%20Reference) (OtherActor :type Actor%20Object%20Reference) (OtherComp :type Primitive%20Component%20Object%20Reference) (OtherBodyIndex :type Integer) (bFromSweep :type Boolean) (SweepResult :type Hit%20Result%20Structure%20%28by%20ref%29))
  ;[1 1 1] If overlapping actor is player, execute the overlap event.
  (if (== OtherActor (Variables|Components|GetPawn))
    (CallFunction|OverlapEvent)))

(event OnComponentEndOverlap(AreaSphere)
  (params (OverlappedComponent :type Primitive%20Component%20Object%20Reference) (OtherActor :type Actor%20Object%20Reference) (OtherComp :type Primitive%20Component%20Object%20Reference) (OtherBodyIndex :type Integer))
  (bind _localmapmanager (Variables|Default|GetLocalMapManager))
  (if (== OtherActor (Game|Player|GetPlayerPawn 0))
    (Utilities|IsValid _localmapmanager
      (:Is%20Valid
        (bind _location (Class|BPIntQuestMapGeneric|GetActiveLocation(Message) _localmapmanager))
        (if (== _location self)
          (Default|SetLocation _localmapmanager)
          (Default|UpdateLocation _localmapmanager))))))

(event OnComponentEndOverlap(AreaCube)
  (params (OverlappedComponent :type Primitive%20Component%20Object%20Reference) (OtherActor :type Actor%20Object%20Reference) (OtherComp :type Primitive%20Component%20Object%20Reference) (OtherBodyIndex :type Integer))
  (bind _localmapmanager (Variables|Default|GetLocalMapManager))
  (if (== OtherActor (Game|Player|GetPlayerPawn 0))
    (Utilities|IsValid _localmapmanager
      (:Is%20Valid
        (bind _location (Class|BPIntQuestMapGeneric|GetActiveLocation(Message) _localmapmanager))
        (if (== _location self)
          (Default|SetLocation _localmapmanager)
          (Default|UpdateLocation _localmapmanager))))))

(event Custom|PlayerIsOverlapping
  ;[1 1 1] Execute overlap event.
  (CallFunction|OverlapEvent))

(event EventBeginPlay
  (bind (_compassmanager _localmapmanager _worldmapmanager) (Class|BPIntQuestMapController|GetComponents(Message) (Game|GetPlayerController 0)))
  (Utilities|IsValid _localmapmanager
    (:Is%20Valid
      (bind _asc_manager__local_map (Utilities|Casting|CastToC_Manager-LocalMap _localmapmanager)
        (:then
          (Variables|Default|SetLocalMapManager _asc_manager__local_map))
        (:CastFailed
          _)))
    (:Is%20Not%20Valid
      _))
  (Utilities|IsValid _worldmapmanager
    (:Is%20Valid
      (bind _asc_manager__world_map (Utilities|Casting|CastToC_Manager-LargeMap _worldmapmanager)
        (:then
          (Variables|Default|SetWorldMapManager _asc_manager__world_map))
        (:CastFailed
          _)))
    (:Is%20Not%20Valid
      _))
  (Variables|Components|SetPawn (Game|Player|GetPlayerPawn 0)) ; Save a reference to the player pawn.
)

(fn ConstructionScript
  (bind _triggersize (Variables|LocationDetails|GetTriggerSize))
  (if (Variables|LocationDetails|GetUseCubeCollision)
    (CallFunction|CollisionSwitch true _triggersize true)
    (CallFunction|CollisionSwitch false 0.0 false)
    (else
      (CallFunction|CollisionSwitch true _triggersize false)
      (CallFunction|CollisionSwitch false 0.0 true))))

(fn CollisionSwitch
  (params (Enable :type Boolean) (Size :type Float%20%28single-precision%29) (UseSphere :type Boolean))
  (bind _areasphere (Variables|Components|GetAreaSphere))
  (bind _areacube (Variables|Components|GetAreaCube))
  (bind _areasphere_2 (Variables|Components|GetAreaSphere))
  (bind _areacube_2 (Variables|Components|GetAreaCube))
  (if Enable
    (if UseSphere
      ;[1 1 1] Set cube extent, enable collision and visibility.
      (Components|Box|SetBoxExtent _areacube (Math|Conversions|ToVector(Float) Size) true)
      (Collision|SetCollisionEnabled _areacube "QueryOnly")
      (Rendering|SetVisibility _areacube true false)
      (else
        ;[1 1 1] Set sphere radius, enable collision and visibility.
        (Components|Sphere|SetSphereRadius _areasphere_2 Size true)
        (Collision|SetCollisionEnabled _areasphere_2 "QueryOnly")
        (Rendering|SetVisibility _areasphere_2 true false)))
    (elif UseSphere
      ;[1 1 1] Set cube extent, disable collision and hide the volume.
      (Components|Box|SetBoxExtent _areacube_2 (Math|Conversions|ToVector(Float) Size) true)
      (Collision|SetCollisionEnabled _areacube_2 "NoCollision")
      (Rendering|SetVisibility _areacube_2 false false)
      (else
        ;[1 1 1] Set sphere radius, disable collision and hide the volume.
        (Components|Sphere|SetSphereRadius _areasphere Size true)
        (Collision|SetCollisionEnabled _areasphere "NoCollision")
        (Rendering|SetVisibility _areasphere false false)))))

(fn OverlapEvent
  (bind _localmapmanager (Variables|Default|GetLocalMapManager))
  (bind _worldmapmanager (Variables|Default|GetWorldMapManager))
  ;[1 1 1] Has this location been discovered?
  (if (Variables|MapData|GetIsDiscovered)
    _
    (else
      ;[1 1 1] Set the location to discovered, display it, and notify the player of it's discovery.
      (Variables|MapData|SetIsDiscovered true)
      (Variables|MapData|SetDisplay true)
      (Development|PrintString (Utilities|String|Append "Area \"" (Utilities|String|ToString(Text) (Variables|LocationDetails|GetLocationName)) "\" discovered by player. Now available for fast travel."))))
  ;[1 1 1] Set current location to active, and update all map markers.
  (Default|SetLocation _localmapmanager self)
  (Default|UpdateLocation _localmapmanager)
  (Default|GetLocations _worldmapmanager)
  (Default|AddMarkers _worldmapmanager))